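; BP_LightSwitch is an interactable switch that toggles a point light on and off.
; On BeginPlay it caches the PointLightComponent from its referenced Light actor.
; Interact waits briefly, then flips that component's visibility using an IsLightOff flag, guarded by a validity check.
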(event `self.ReceiveBeginPlay`
  (`self.SetLightRef`))

(event `/Game/FirstPerson/Blueprints/Interfaces/BPI_Interactable.Interact`
  (`KismetSystemLibrary.Delay` 0.4)
  (`self.LightFunctions`))

(fn `LightFunctions`
  (`self.PointLight`
    (:`then`
      (if (`self.IsLightOff?`)
        (`SceneComponent.SetVisibility` (`self.PointLight`) true false)
        (set `self.IsLightOff?` false)
        (else
          (`SceneComponent.SetVisibility` (`self.PointLight`) false false)
          (set `self.IsLightOff?` true))))
    (:`else`)))

(fn `SetLightRef`
  (set `self.PointLight` (`self.GetComponentByClass` (`self.Light`) "/Script/Engine.PointLightComponent")))

(fn `UserConstructionScript`)